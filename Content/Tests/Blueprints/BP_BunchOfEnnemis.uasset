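; BP_BunchOfEnnemis is a test Blueprint that places a group of aliens along a spline.
; Its construction script loops over the spline point indices and adds a child actor component for each.
; Each child takes the point's local location, rotation and scale, with EnnemisZAxis added to the yaw to offset its facing.
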(fn `UserConstructionScript`
  (bind _spline (`self.Spline`))
  ;[1 1 1] creates new aliens
  (for _index (range (+ (`SplineComponent.GetNumberOfSplinePoints` _spline) 1))
    (`AddComponent|NODE_AddChildActorComponent-0` :`RelativeTransform` (`KismetMathLibrary.MakeTransform` (.location (`SplineComponent.GetTransformAtSplinePoint` _spline _index "Local" false)) (`KismetMathLibrary.MakeRotator` (.roll (.rotation (`SplineComponent.GetTransformAtSplinePoint` _spline _index "Local" false))) (.pitch (.rotation (`SplineComponent.GetTransformAtSplinePoint` _spline _index "Local" false))) (+ (.yaw (.rotation (`SplineComponent.GetTransformAtSplinePoint` _spline _index "Local" false))) (`self.EnnemisZAxis`))) (.scale (`SplineComponent.GetTransformAtSplinePoint` _spline _index "Local" false))))))