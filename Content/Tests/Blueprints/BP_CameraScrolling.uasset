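; Test auto-scrolling camera actor that becomes player 0's view target on BeginPlay and limits how far players can go.
; Each tick it asks the game mode whether it can move, then shifts the camera along local Y by Speed, unscaled by delta time.
; The construction script attaches a configurable hitbox to the camera as a player barrier, negating camera pitch and roll and using its own yaw.
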(event `self.ReceiveTick`
  (params (DeltaSeconds :type "Float (single-precision)"))
  ;[1 1 1] Movement
  (bind _canmove (message `/Game/Tests/Blueprints/Interface/BPI_GameMode.CameraCanMove` (`GameplayStatics.GetGameMode`)))
  (if _canmove
    (`SceneComponent.K2_AddLocalOffset` (`self.Camera`) (`KismetMathLibrary.MakeVector` 0.0 (`self.Speed`)) false false)))

(event `self.ReceiveBeginPlay`
  ;[1 1 1] Set to main camera
  (`PlayerController.SetViewTargetWithBlend` (`GameplayStatics.GetPlayerController` 0) self 0.0 "VTBlend_Cubic" 0.0 false))

(fn `UserConstructionScript`
  ;[1 1 1] Creates a hitbox to prevent the players to go beyond the camera. (The position can change and the size of it too)
  (bind _returnvalue (`AddComponent|NODE_AddBoxComponent-0` :`RelativeTransform` (`KismetMathLibrary.MakeTransform` (`self.HitboxPosition`) (`KismetMathLibrary.MakeRotator` (* (.roll (`SceneComponent.K2_GetComponentRotation` (`self.Camera`))) -1.0) (* (.pitch (`SceneComponent.K2_GetComponentRotation` (`self.Camera`))) -1.0) (`self.KitboxZRot`)))))
  (`BoxComponent.SetBoxExtent` _returnvalue (`self.HitBox Extent`) true)
  (`SceneComponent.K2_AttachToComponent` _returnvalue (`self.Camera`) "None" "KeepRelative" "KeepRelative" "KeepRelative" true))