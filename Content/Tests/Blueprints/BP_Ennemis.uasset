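; Test enemy that moves along with the game mode's scrolling speed and kills actors implementing BPI_Player when its capsule hits them.
; Each Tick, while the game mode lets the camera move, it advances on local X with sweep.
; FrontBox and GroundBox overlaps set flags that add unswept offsets: forward and up to jump obstacles, backward and down when off the ground.
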(event `self.Capsule.OnComponentHit`
  (params (HitComponent :type "PrimitiveComponent Object Reference") (OtherActor :type "Actor Object Reference") (OtherComp :type "PrimitiveComponent Object Reference") (NormalImpulse :type "Vector Structure") (Hit :type "HitResult Structure (by ref)"))
  ;[1 1 1] Kill on impact
  (bind _outactors (`GameplayStatics.GetAllActorsWithInterface` "/Game/Tests/Blueprints/Interface/BPI_Player.BPI_Player_C"))
  (if (`KismetArrayLibrary.Array_IsValidIndex` _outactors (`KismetArrayLibrary.Array_Find` _outactors OtherActor))
    (message `/Game/Tests/Blueprints/Interface/BPI_Player.Death` OtherActor)))

(event `self.ReceiveTick`
  (params (DeltaSeconds :type "Float (single-precision)"))
  (bind _returnvalue (`GameplayStatics.GetGameMode`))
  ;[1 1 1] Movement
  (bind _canmove (message `/Game/Tests/Blueprints/Interface/BPI_GameMode.CameraCanMove` _returnvalue))
  (bind _scrollingspeed (message `/Game/Tests/Blueprints/Interface/BPI_GameMode.Get Scrolling Speed` _returnvalue))
  (if _canmove
    (bind _returnvalue_2 (`KismetMathLibrary.MakeVector` _scrollingspeed))
    (`self.K2_AddActorLocalOffset` _returnvalue_2 true)
    (`|ExecutionSequence`
      (:`then_0`
        ;[1 1 1] Jumps
        (if (`self.GoesUp`)
          (bind _returnvalue_3 (+ _returnvalue_2 (0.0 0.0 7.0)))
          (`self.K2_AddActorLocalOffset` _returnvalue_3)))
      (:`then_1`
        ;[1 1 1] Fall
        (if (not (`self.OnGround`))
          (`self.K2_AddActorLocalOffset` (* _returnvalue_3 -1)))))))

(event `self.FrontBox.OnComponentBeginOverlap`
  (params (OverlappedComponent :type "PrimitiveComponent Object Reference") (OtherActor :type "Actor Object Reference") (OtherComp :type "PrimitiveComponent Object Reference") (OtherBodyIndex :type Integer) (bFromSweep :type Boolean) (SweepResult :type "HitResult Structure (by ref)"))
  ;[1 1 1] Front collision
  (set `self.GoesUp` true))

(event `self.FrontBox.OnComponentEndOverlap`
  (params (OverlappedComponent :type "PrimitiveComponent Object Reference") (OtherActor :type "Actor Object Reference") (OtherComp :type "PrimitiveComponent Object Reference") (OtherBodyIndex :type Integer))
  ;[1 1 1] Front collision
  (set `self.GoesUp` false))

(event `self.GroundBox.OnComponentBeginOverlap`
  (params (OverlappedComponent :type "PrimitiveComponent Object Reference") (OtherActor :type "Actor Object Reference") (OtherComp :type "PrimitiveComponent Object Reference") (OtherBodyIndex :type Integer) (bFromSweep :type Boolean) (SweepResult :type "HitResult Structure (by ref)"))
  ;[1 1 1] Ground collision
  (set `self.OnGround` true))

(event `self.GroundBox.OnComponentEndOverlap`
  (params (OverlappedComponent :type "PrimitiveComponent Object Reference") (OtherActor :type "Actor Object Reference") (OtherComp :type "PrimitiveComponent Object Reference") (OtherBodyIndex :type Integer))
  ;[1 1 1] Ground collision
  (set `self.OnGround` false))

(fn `UserConstructionScript`)