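; GM_TestPlayer is a test game mode that spawns local players and puts the first player controller on a scrolling camera.
; On BeginPlay it calls CreatePlayer in a loop driven by NumberOfPlayers, then finds the BP_CameraScrolling actor and blends the view target to it.
; A check that would reset out-of-range player counts to five exists but is not connected, so it never runs.
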(event `self.ReceiveBeginPlay`
  ;[1 1 1] Creates the players
  (for _ (range (+ (`self.NumberOfPlayers`) 1))
    (`GameplayStatics.CreatePlayer` -1))
  (bind _returnvalue (`GameplayStatics.GetActorOfClass` "/Game/Tests/Blueprints/BP_CameraScrolling.BP_CameraScrolling_C"))
  (set `Actor.bFindCameraComponentWhenViewTarget` true _returnvalue)
  (`PlayerController.SetViewTargetWithBlend` (`GameplayStatics.GetPlayerController` 0) _returnvalue 0.0 "VTBlend_Cubic" 0.0 false))

(fn `UserConstructionScript`)